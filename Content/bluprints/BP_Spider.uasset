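; BP_Spider is an actor that periodically hands player control to a randomly chosen character.
; Tick turns its StaticMesh to the CameraBoom's target yaw, then runs a 2-second Delay that acts as a repeating timer for Swap.
; Swap unpossesses the current pawn of player controller 0 and possesses the first Char1 or Char2 found in the level, picked at random.
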(event Custom|swap
  (bind _returnvalue (Game|GetPlayerController 0))
  (Pawn|UnPossess _returnvalue)
  (switch int (Math|Random|RandomIntegerinRange 0 1)
    (:0
      (bind _outactors (Actor|GetAllActorsOfClass (Variables|Default|Getchar1)))
      (Pawn|Possess _returnvalue (Utilities|Array|Get(acopy) _outactors)))
    (:1
      (bind _outactors_2 (Actor|GetAllActorsOfClass (Variables|Default|Getchar2)))
      (Pawn|Possess _returnvalue (Utilities|Array|Get(acopy) _outactors_2)))))

(event EventBeginPlay)

(event Collision|EventActorBeginOverlap
  (params (OtherActor :type Actor%20Object%20Reference)))

(event EventTick
  (params (DeltaSeconds :type Float%20%28single-precision%29))
  (Transformation|SetRelativeRotation (Variables|Default|GetStaticMesh) (Math|Rotator|MakeRotator 0.0 0.0 (.Yaw (Math|Rotator|BreakRotator (Class|SpringArmComponent|GetTargetRotation (Variables|Default|GetcameraBoom))))) false false)
  (Utilities|FlowControl|Delay 2.0)
  (CallFunction|Swap))

(fn ConstructionScript)